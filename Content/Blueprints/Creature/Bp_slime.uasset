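; Slime enemy creature that chases the player and attacks at close range, built on a parent creature class.
; BeginPlay loads its stats from the "Smile" row of CreatureDT before running parent setup.
; Each tick runs a small state machine: Idle acquires Bp_player, Move attacks within range or picks a four-way facing from the dominant X/Z axis.
; It destroys itself when Hp equals zero.
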(event `self.ReceiveBeginPlay`
  (bind _returnvalue (`|GetDataTableRow` "/Game/Blueprints/Data/CreatureDT.CreatureDT" "Smile")
    (:`then`
      (set `self.Data` _returnvalue)
      (`parent.ReceiveBeginPlay`))))

(event `self.ReceiveTick`
  (params (DeltaSeconds :type "Float (single-precision)"))
  (`parent.ReceiveTick` DeltaSeconds)
  (`self.UpdateAi`)
  (if (== (`self.Hp`) 0)
    (`self.K2_DestroyActor`)))

(fn `UpdateAi`
  (bind _target (`self.Target`))
  (bind (_chasedirection_x _chasedirection_y _chasedirection_z) (`KismetMathLibrary.BreakVector` (`self.ChaseDirection`)))
  (switch `/Game/Blueprints/Struct/Estate` (`self.State`)
    (:`NewEnumerator0`
      (bind _returnvalue (`GameplayStatics.GetActorOfClass` "/Game/Blueprints/Creature/Bp_player.Bp_player_C"))
      (bind _output_get (set `self.Target` _returnvalue))
      (`/Engine/EditorBlueprintResources/StandardMacros.IsValid` _output_get
        (:`Is Valid`
          (set `self.State` "NewEnumerator1"))))
    (:`NewEnumerator1`
      (`/Engine/EditorBlueprintResources/StandardMacros.IsValid` _target
        (:`Is Valid`
          (bind _output_get_2 (set `self.ChaseDirection` (- (`self.K2_GetActorLocation` _target) (`self.K2_GetActorLocation`))))
          (if (< (`KismetMathLibrary.VSize` _output_get_2) 20.0)
            (`self.BeginAtk`)
            (elif (> (`KismetMathLibrary.Abs` _chasedirection_x) (`KismetMathLibrary.Abs` _chasedirection_z))
              (`/Engine/EditorBlueprintResources/StandardMacros.CompareFloat` _chasedirection_x
                (:`>`
                  (set `self.Direction` "NewEnumerator3"))
                (:`<`
                  (set `self.Direction` "NewEnumerator2")))
              (else
                (`/Engine/EditorBlueprintResources/StandardMacros.CompareFloat` _chasedirection_z
                  (:`>`
                    (set `self.Direction` "NewEnumerator0"))
                  (:`<`
                    (set `self.Direction` "NewEnumerator1")))))))))))

(fn `UserConstructionScript`
  (`parent.UserConstructionScript`))