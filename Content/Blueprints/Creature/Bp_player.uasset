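; Player creature Blueprint that turns movement and attack input into creature state and facing.
; BeginPlay loads the "Player" row from CreatureDT into Data and only runs parent initialization if the row is found.
; UpdateInput, active only in Idle or Move, switches between those states and sets Direction from the move axes, with horizontal overriding vertical.
; The Attack press calls BeginAtk.
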(event `self.ReceiveBeginPlay`
  (bind _returnvalue (`|GetDataTableRow` "/Game/Blueprints/Data/CreatureDT.CreatureDT" "Player")
    (:`then`
      (set `self.Data` _returnvalue)
      (`parent.ReceiveBeginPlay`))))

(event `self.ReceiveTick`
  (params (DeltaSeconds :type "Float (single-precision)"))
  (`parent.ReceiveTick` DeltaSeconds))

(event `InputAction|Attack`
  (params (Key :type "Key Structure"))
  (:`Pressed`
    (`self.BeginAtk`)))

(fn `Update Input`
  (switch `/Game/Blueprints/Struct/Estate` (`self.State`)
    (:`NewEnumerator0`
      _)
    (:`NewEnumerator1`
      _))
  (`|ExecutionSequence`
    (:`then_0`
      (if (or (!= (`self.GetInputAxisValue`) 0.0) (!= (`self.GetInputAxisValue`) 0.0))
        (set `self.State` "NewEnumerator1")
        (else
          (set `self.State` "NewEnumerator0"))))
    (:`then_1`
      (`/Engine/EditorBlueprintResources/StandardMacros.CompareFloat` (`self.GetInputAxisValue`)
        (:`>`
          (set `self.Direction` "NewEnumerator0"))
        (:`<`
          (set `self.Direction` "NewEnumerator1"))))
    (:`then_2`
      (`/Engine/EditorBlueprintResources/StandardMacros.CompareFloat` (`self.GetInputAxisValue`)
        (:`>`
          (set `self.Direction` "NewEnumerator3"))
        (:`<`
          (set `self.Direction` "NewEnumerator2"))))))

(fn `UserConstructionScript`)