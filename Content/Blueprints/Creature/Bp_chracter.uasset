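; Base 2D Paper2D character Blueprint with four-directional movement, melee attacks and health, configured through a Data asset for HP and flipbooks.
; Tick moves it along its Direction while in Move state and picks the flipbook by state and direction, flipping the side sprite for left.
; BeginAtk damages other Bp_chracter actors overlapping the directional range, then returns to Move after the flipbook's length.
; OnDamaged clamps HP and updates the HP bar widget.
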(event `self.ReceiveBeginPlay`
  (bind _output_get (set `self.Hp` (`.Hp_24_70426A7943E76B11A54DEB8B9ED68BD5` (break `/Game/Blueprints/Data/CreatureData` (`self.Data`)))))
  (set `self.MaxHp` _output_get))

(event `self.ReceiveTick`
  (params (DeltaSeconds :type "Float (single-precision)"))
  (`self.UpdateLogic`)
  (`self.UpdateAnimation`))

(event `BeginAtk`
  (switch `/Game/Blueprints/Struct/Estate` (`self.State`)
    (:`NewEnumerator0`
      _)
    (:`NewEnumerator1`
      _))
  (set `self.State` "NewEnumerator2")
  (`self.UpdateAnimation`)
  (`self.ProcessAtk`)
  (`KismetSystemLibrary.Delay` (`PaperFlipbookComponent.GetFlipbookLength` (`self.Sprite`)))
  (set `self.State` "NewEnumerator1"))

(fn `OnDamaged`
  (params (Damage :type Integer) (Attacker :type "/Game/Blueprints/Creature/Bp_chracter Object Reference"))
  (bind _maxhp (`self.MaxHp`))
  (if (not (== self Attacker))
    (bind _output_get (set `self.Hp` (`KismetMathLibrary.Clamp` (- (`self.Hp`) Damage) 0 _maxhp)))
    (bind _aswbp_hpbar (cast `/Game/Blueprints/WBP_Hpbar` (`WidgetComponent.GetUserWidgetObject` (`self.HpBarwidget`))))
    (set `/Game/Blueprints/WBP_Hpbar.HpRate` (/ _output_get (`KismetMathLibrary.Conv_IntToDouble` _maxhp)) _aswbp_hpbar)))

(fn `ProcessAtk`
  (bind _atkrange_side (`self.AtkRange_side`))
  (for _array_element (`PrimitiveComponent.GetOverlappingActors` (select `/Game/Blueprints/Struct/Edirection` (`self.Direction`) :`NewEnumerator0` (`self.AtkRange_up`) :`NewEnumerator1` (`self.AtkRange_down`) :`NewEnumerator2` _atkrange_side :`NewEnumerator3` _atkrange_side) "Bp_chracter_C")
    (bind _asbp_creature (cast `/Game/Blueprints/Creature/Bp_chracter` _array_element))
    (if (not (== self _asbp_creature))
      (`self.OnDamaged` _asbp_creature 10 self))))

(fn `UpdateAnimation`
  (bind (_data_hp _data_damage _data_up_idle _data_down_idle _data_side_idle _data_up_move _data_down_move _data_side_move _data_up_atk _data_down_atk _data_side_atk) (break `/Game/Blueprints/Data/CreatureData` (`self.Data`)))
  (`SceneComponent.K2_SetRelativeRotation` (`self.Sprite`) (select `bool` (`|EnumEquality` (`self.Direction`) "NewEnumerator2") :`true` (struct :`Yaw` 180.0) :!type "Rotator Structure") false false)
  (switch `/Game/Blueprints/Struct/Estate` (`self.State`)
    (:`NewEnumerator0`
      (`PaperFlipbookComponent.SetFlipbook` (`self.Sprite`) (select `/Game/Blueprints/Struct/Edirection` (`self.Direction`) :`NewEnumerator0` _data_up_idle :`NewEnumerator1` _data_down_idle :`NewEnumerator2` _data_side_idle :`NewEnumerator3` _data_side_idle)))
    (:`NewEnumerator1`
      (`PaperFlipbookComponent.SetFlipbook` (`self.Sprite`) (select `/Game/Blueprints/Struct/Edirection` (`self.Direction`) :`NewEnumerator0` _data_up_move :`NewEnumerator1` _data_down_move :`NewEnumerator2` _data_side_move :`NewEnumerator3` _data_side_move)))
    (:`NewEnumerator2`
      (`PaperFlipbookComponent.SetFlipbook` (`self.Sprite`) (select `/Game/Blueprints/Struct/Edirection` (`self.Direction`) :`NewEnumerator0` _data_up_atk :`NewEnumerator1` _data_down_atk :`NewEnumerator2` _data_side_atk :`NewEnumerator3` _data_side_atk)))))

(fn `UpdateLogic`
  (switch `/Game/Blueprints/Struct/Estate` (`self.State`)
    (:`NewEnumerator1`
      (`self.AddMovementInput` (select `/Game/Blueprints/Struct/Edirection` (`self.Direction`) :`NewEnumerator0` (0.0 0.0 1.0) :`NewEnumerator1` (0.0 0.0 -1.0) :`NewEnumerator2` (-1.0 0.0 0.0) :`NewEnumerator3` (1.0 0.0 0.0) :!type "Vector Structure")))))

(fn `UserConstructionScript`)